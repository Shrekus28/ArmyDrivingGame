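; BP_SUV is a drivable SUV vehicle pawn from the Vehicle Variety Pack.
; Input axes feed throttle and steering into its VehicleMovement component, and Space Bar holds the handbrake.
; Look and turn axes drive controller pitch and yaw, with pitch inverted.
; Holding left mouse lets the spring arm follow control rotation, giving a click-to-orbit camera.
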(event Input|AxisEvents|InputAxisMoveForward
  (params (AxisValue :type Float%20%28single-precision%29))
  (Class|WheeledVehicleMovementComponent|SetThrottleInput (Variables|Default|GetVehicleMovement) AxisValue))

(event Input|AxisEvents|InputAxisMoveRight
  (params (AxisValue :type Float%20%28single-precision%29))
  (Class|WheeledVehicleMovementComponent|SetSteeringInput (Variables|Default|GetVehicleMovement) AxisValue))

(event Input|AxisEvents|InputAxisLookUp
  (params (AxisValue :type Float%20%28single-precision%29))
  (Pawn|Input|AddControllerPitchInput (* AxisValue -1.0)))

(event Input|AxisEvents|InputAxisTurn
  (params (AxisValue :type Float%20%28single-precision%29))
  (Pawn|Input|AddControllerYawInput AxisValue))

(event Input|KeyboardEvents|SpaceBar
  (params (Key :type Key%20Structure :default "None"))
  (bind _vehiclemovement (Variables|Default|GetVehicleMovement))
  (:Pressed
    (Class|WheeledVehicleMovementComponent|SetHandbrakeInput _vehiclemovement true))
  (:Released
    (Class|WheeledVehicleMovementComponent|SetHandbrakeInput _vehiclemovement false)))

(event Input|MouseEvents|LeftMouseButton
  (params (Key :type Key%20Structure :default "None"))
  (bind _springarm (Variables|Components|GetSpringArm))
  (:Pressed
    (Variables|/Script/Engine.SpringArmComponent|SetbUsePawnControlRotation _springarm true))
  (:Released
    (Variables|/Script/Engine.SpringArmComponent|SetbUsePawnControlRotation _springarm false)))

(fn ConstructionScript)