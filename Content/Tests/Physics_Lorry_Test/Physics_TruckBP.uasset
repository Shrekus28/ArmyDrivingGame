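; Physics test truck Blueprint that pushes its Chassis component with forces.
; Accelerate applies Speed-scaled force against the chassis forward vector for positive input and along it for negative input, using only the sign.
; BeginPlay calls it once with a positive value, so the push is not sustained.
; MoveForward and Tick are empty, and Turn feeds an empty Steering event.
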(event Custom|Accelerate
  (params (Axis%20Value :type Float%20%28single-precision%29))
  (bind _chassis (Variables|Default|GetChassis))
  (Utilities|FlowControl|Sequence
    (:then_0
      (if (> Axis%20Value 0.0)
        (Physics|AddForce _chassis (* (Math|Vector|NegateVector (Math|Vector|GetForwardVector _chassis)) (Variables|Default|GetSpeed)) "None" false)))
    (:then_1
      (if (< Axis%20Value 0.0)
        (Physics|AddForce _chassis (* (Math|Vector|GetForwardVector (Variables|Default|GetChassis)) (Variables|Default|GetSpeed)) "None" false)))))

(event Custom|Steering
  (params (Axis%20Value :type Float%20%28single-precision%29)))

(event EventTick
  (params (DeltaSeconds :type Float%20%28single-precision%29)))

(event EventBeginPlay
  (CallFunction|Accelerate 0.1))

(event Input|AxisEvents|InputAxisTurn
  (params (AxisValue :type Float%20%28single-precision%29))
  (CallFunction|Steering AxisValue))

(event Input|AxisEvents|InputAxisMoveForward
  (params (AxisValue :type Float%20%28single-precision%29)))

(fn ConstructionScript)