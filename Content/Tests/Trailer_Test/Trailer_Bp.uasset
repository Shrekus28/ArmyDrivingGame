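; Test trailer Blueprint with a Stand component that can be removed or placed back.
; RemoveStand and PlaceStand toggle its visibility and collision rather than destroying it, update IsStandRemoved, and both fire the StandRemoved dispatcher.
; A check event calls RemoveStand while Stand is valid, otherwise printing once that it is gone.
; The code binding a handler to StandRemoved is unconnected and never runs.
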(event Custom|Make%20sure%20sta\nd%20is%20removed
  (Utilities|IsValid (Variables|Default|GetStand)
    (:Is%20Valid
      (Development|PrintString "stand syill there")
      (CallFunction|RemoveStand))
    (:Is%20Not%20Valid
      (Utilities|FlowControl|DoOnce false
        (:Completed
          (Development|PrintString "stand removed"))))))

(event EventTick
  (params (DeltaSeconds :type Float%20%28single-precision%29)))

(fn ConstructionScript)

(fn RemoveStand
  (bind _stand (Variables|Default|GetStand))
  (Rendering|SetVisibility _stand false false)
  (Collision|SetCollisionEnabled _stand "NoCollision")
  (Variables|Default|SetbIs%20Stand%20Removed true)
  (Default|CallStandRemoved))

(fn PlaceStand
  (bind _stand (Variables|Default|GetStand))
  (Rendering|SetVisibility _stand true false)
  (Collision|SetCollisionEnabled _stand "QueryAndPhysics")
  (Variables|Default|SetbIs%20Stand%20Removed false)
  (Default|CallStandRemoved))