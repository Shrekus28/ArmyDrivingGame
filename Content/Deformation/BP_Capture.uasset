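; Scene capture actor for a deformation effect that follows the player and maintains a persistent render target.
; On BeginPlay it clears both render targets and writes the capture size to MPC_Capture.
; Each tick it moves in XY, snapped to 1/256th-of-ortho-width texels to avoid shimmering, and publishes its location to the collection.
; It then draws M_DrawToPersistent into PersistentRT with the normalized move offset, keeping accumulated data aligned as the window scrolls.
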(event EventBeginPlay
  (Rendering|Material|SetScalarParameterValue "/Game/Deformation/MPC_Capture.MPC_Capture" "Capture Size" (Variables|/Script/Engine.SceneCaptureComponent2D|GetOrthoWidth (Variables|Default|GetSceneCaptureComponent2D)) :!class /Script/Engine.KismetMaterialLibrary)
  (bind _returnvalue (Rendering|Material|CreateDynamicMaterialInstance "/Game/Deformation/M_DrawToPersistent.M_DrawToPersistent" "None" :!class /Script/Engine.KismetMaterialLibrary))
  (Variables|Default|SetDraw%20Material _returnvalue)
  (Rendering|ClearRenderTarget2D "/Game/Deformation/staticRTCapture.staticRTCapture")
  (Rendering|ClearRenderTarget2D "/Game/Deformation/persistentRT.persistentRT"))

(event EventTick
  (params (DeltaSeconds :type Float%20%28single-precision%29))
  (CallFunction|MoveCapture)
  (CallFunction|DrawtoPersistent))

(fn ConstructionScript)

(fn DrawtoPersistent
  (bind _move_offset (Variables|Default|GetMove%20Offset))
  (bind _scenecapturecomponent2d (Variables|Default|GetSceneCaptureComponent2D))
  (bind _orthowidth (Variables|/Script/Engine.SceneCaptureComponent2D|GetOrthoWidth _scenecapturecomponent2d))
  (bind _returnvalue (/ _move_offset _orthowidth))
  (Rendering|Material|SetVectorParameterValue (Variables|Default|GetDraw%20Material) "Offset" (Utilities|Struct|MakeLinearColor (.x _returnvalue) (.y _returnvalue) 0.0 1.0) :!class /Script/Engine.MaterialInstanceDynamic)
  (Rendering|DrawMaterialtoRenderTarget "/Game/Deformation/persistentRT.persistentRT" (Variables|Default|GetDraw%20Material)))

(fn MoveCapture
  (bind _returnvalue (Game|Player|GetPlayerPawn 0))
  (bind _returnvalue_2 (/ 1.0 256.0))
  (bind _returnvalue_3 (Transformation|GetActorLocation))
  (bind _scenecapturecomponent2d (Variables|Default|GetSceneCaptureComponent2D))
  (bind _returnvalue_4 (Transformation|GetActorLocation _returnvalue))
  (bind _orthowidth (Variables|/Script/Engine.SceneCaptureComponent2D|GetOrthoWidth _scenecapturecomponent2d))
  (bind _returnvalue_5 (* _orthowidth _returnvalue_2))
  (bind _returnvalue_6 (Utilities|SnaptoPixelWorldSize (.x _returnvalue_4) (.y _returnvalue_4) _returnvalue_5))
  (bind _returnvalue_7 (- _returnvalue_6 _returnvalue_3))
  (bind _output_get (Variables|Default|SetMove%20Offset (Math|Vector2D|MakeVector2D (.x _returnvalue_7) (.y _returnvalue_7))))
  (Transformation|AddActorWorldOffset (Math|Vector|MakeVector (.x _output_get) (.y _output_get) 0.0))
  (Rendering|Material|SetVectorParameterValue "/Game/Deformation/MPC_Capture.MPC_Capture" "Capture Location" (Math|Conversions|ToLinearColor(Vector) (Transformation|GetActorLocation)) :!class /Script/Engine.KismetMaterialLibrary))