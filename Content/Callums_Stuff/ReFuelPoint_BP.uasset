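; A refuelling point actor with a limited fuel reserve that tops up vehicles entering its box trigger.
; Overlap by a VehicleParent_BP stores the vehicle and starts a fast looping timer through a DoOnce; leaving resets it and halts refuelling via a flag.
; Each tick of the timer passes fuel to the vehicle's FuelEvent and drains the reserve, until it empties or the vehicle's tank and canisters are full.
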(event OnComponentBeginOverlap(Box)
  (params (OverlappedComponent :type Primitive%20Component%20Object%20Reference) (OtherActor :type Actor%20Object%20Reference) (OtherComp :type Primitive%20Component%20Object%20Reference) (OtherBodyIndex :type Integer) (bFromSweep :type Boolean) (SweepResult :type Hit%20Result%20Structure%20%28by%20ref%29))
  (Utilities|FlowControl|DoOnce false
    (:Completed
      (bind _asvehicle_parent_bp (Utilities|Casting|CastToVehicleParent_BP OtherActor))
      (Variables|Default|SetPlayer%20Vehicle%20Reference _asvehicle_parent_bp)
      (CallFunction|StartFuelTimer)
      (Variables|Default|SetIs%20Refuelling true))))

(event OnComponentEndOverlap(Box)
  (params (OverlappedComponent :type Primitive%20Component%20Object%20Reference) (OtherActor :type Actor%20Object%20Reference) (OtherComp :type Primitive%20Component%20Object%20Reference) (OtherBodyIndex :type Integer))
  (Utilities|Casting|CastToVehicleParent_BP OtherActor)
  (Utilities|FlowControl|Sequence
    (:then_0
      (Utilities|FlowControl|DoOnce false) ; enters at Reset
    )
    (:then_1
      (Variables|Default|SetIs%20Refuelling false))))

(event Custom|Start%20Fuel%20Timer
  (Utilities|Time|SetTimerbyEvent (delegate Custom|Add%20Fuel) 0.01 true))

(event Custom|Add%20Fuel
  (bind _player_vehicle_reference (Variables|Default|GetPlayer%20Vehicle%20Reference))
  (bind _player_vehicle_reference_2 (Variables|Default|GetPlayer%20Vehicle%20Reference))
  (if (Variables|Default|GetIs%20Refuelling)
    (if (not (<= (Variables|Default|GetCurrent%20Fuel%20Amount) 0.0))
      (if (>= (Variables|/Game/Callums_Stuff/VehicleParent_BP.VehicleParent_BP_C|GetCurrent%20Fuel%20Amount _player_vehicle_reference) (Variables|/Game/Callums_Stuff/VehicleParent_BP.VehicleParent_BP_C|GetMaximum%20Fuel%20Capacity _player_vehicle_reference))
        (if (< (Variables|/Game/Callums_Stuff/VehicleParent_BP.VehicleParent_BP_C|GetCurrent%20Fuel%20Canisters%20Held%20 _player_vehicle_reference_2) (Variables|/Game/Callums_Stuff/VehicleParent_BP.VehicleParent_BP_C|GetFuel%20Canisters%20Held%20Maximum _player_vehicle_reference_2))
          (Default|FuelEvent (Variables|Default|GetPlayer%20Vehicle%20Reference) (Variables|Default|GetFuel%20Given%20to%20Player) :!label _label)
          (Variables|Default|SetCurrent%20Fuel%20Amount (- (Variables|Default|GetCurrent%20Fuel%20Amount) (Variables|Default|GetFuel%20Given%20to%20Player)))
          (if (<= (Variables|Default|GetCurrent%20Fuel%20Amount) 0.0)
            (Variables|Default|SetCurrent%20Fuel%20Amount 0.0)))
        (else
          (goto _label))))))

(event EventBeginPlay)

(event Collision|EventActorBeginOverlap
  (params (OtherActor :type Actor%20Object%20Reference)))

(event EventTick
  (params (DeltaSeconds :type Float%20%28single-precision%29)))

(fn ConstructionScript)