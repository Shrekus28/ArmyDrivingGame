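; IED explosion actor that applies ExplosionDamage to vehicles overlapping it.
; On begin overlap, a sequence tries casts to OLDParent_BP, ParentVehicle_BP and 6_wheel_Test, storing each match.
; The first two branches call HealthDamageEvent on the cast vehicle; the 6-wheel branch calls it without targeting its stored reference.
; Tick prints the name of the Sphere's first overlapping component as debug output.
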(event Collision|EventActorBeginOverlap
  (params (OtherActor :type Actor%20Object%20Reference))
  (Utilities|FlowControl|Sequence
    (:then_0
      (bind _asoldparent_bp (Utilities|Casting|CastToOLDParent_BP OtherActor))
      (bind _output_get (Variables|Default|SetPlayer%20Vehicle%20Reference _asoldparent_bp))
      (Default|Health/DamageEvent _output_get (Variables|Default|GetExplosion%20Damage) 0.0))
    (:then_1
      (bind _asparent_vehicle_bp (Utilities|Casting|CastToParentVehicle_BP OtherActor))
      (bind _output_get_2 (Variables|Default|SetNew%20Player%20Vehicle%20Reference _asparent_vehicle_bp))
      (Default|Health/DamageEvent _output_get_2 (Variables|Default|GetExplosion%20Damage) 0.0))
    (:then_2
      (bind _as6_wheel_test (Utilities|Casting|CastTo6_wheel_Test OtherActor))
      (Variables|Default|Set6%20wheel%20ref _as6_wheel_test)
      (CallFunction|Health/DamageEvent (Variables|Default|GetExplosion%20Damage) 0.0))))

(event EventTick
  (params (DeltaSeconds :type Float%20%28single-precision%29))
  (Development|PrintString (Utilities|GetDisplayName (Utilities|Array|Get(acopy) (Class|PrimitiveComponent|GetOverlappingComponents (Variables|Default|GetSphere))))))

(fn ConstructionScript)