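; Repair kit station that refills an overlapping player vehicle's repair kits from its own limited stock.
; On box begin overlap, it tops the vehicle up to its max or hands over whatever stock remains, deducting that from the station.
; Duplicate branches support OLDParent_BP and the newer ParentVehicle_BP.
; A DoOnce ahead of the casts gates refills and resets only when either vehicle type leaves the box.
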(event OnComponentBeginOverlap(Box)
  (params (OverlappedComponent :type Primitive%20Component%20Object%20Reference) (OtherActor :type Actor%20Object%20Reference) (OtherComp :type Primitive%20Component%20Object%20Reference) (OtherBodyIndex :type Integer) (bFromSweep :type Boolean) (SweepResult :type Hit%20Result%20Structure%20%28by%20ref%29))
  (Utilities|FlowControl|DoOnce false
    (:Completed
      (Utilities|FlowControl|Sequence
        (:then_0
          (bind _asoldparent_bp (Utilities|Casting|CastToOLDParent_BP OtherActor))
          (bind _output_get (Variables|Default|SetPlayer%20Vehicle%20Reference _asoldparent_bp))
          (if (< (Variables|/Game/Callums_Stuff/OLDParent_BP.OLDParent_BP_C|GetRepair%20Kit%20Current _output_get) (Variables|/Game/Callums_Stuff/OLDParent_BP.OLDParent_BP_C|GetRepair%20Kit%20Max _output_get))
            (if (not (<= (Variables|Default|GetRepair%20Kit%20Station%20Stock%20Current) 0.0))
              (Variables|Default|SetVehicle%20Max%20-%20Current%20Difference (- (Variables|/Game/Callums_Stuff/OLDParent_BP.OLDParent_BP_C|GetRepair%20Kit%20Max (Variables|Default|GetPlayer%20Vehicle%20Reference)) (Variables|/Game/Callums_Stuff/OLDParent_BP.OLDParent_BP_C|GetRepair%20Kit%20Current (Variables|Default|GetPlayer%20Vehicle%20Reference))))
              (if (< (- (Variables|Default|GetRepair%20Kit%20Station%20Stock%20Current) (Variables|Default|GetVehicle%20Max%20-%20Current%20Difference)) 0.0)
                (Variables|/Game/Callums_Stuff/OLDParent_BP.OLDParent_BP_C|SetRepair%20Kit%20Current (Variables|Default|GetPlayer%20Vehicle%20Reference) (+ (Variables|Default|GetRepair%20Kit%20Station%20Stock%20Current) (Variables|/Game/Callums_Stuff/OLDParent_BP.OLDParent_BP_C|GetRepair%20Kit%20Current (Variables|Default|GetPlayer%20Vehicle%20Reference))))
                (Variables|Default|SetRepair%20Kit%20Station%20Stock%20Current (- (Variables|Default|GetRepair%20Kit%20Station%20Stock%20Current) (Variables|Default|GetRepair%20Kit%20Station%20Stock%20Current)))
                (else
                  (Variables|/Game/Callums_Stuff/OLDParent_BP.OLDParent_BP_C|SetRepair%20Kit%20Current (Variables|Default|GetPlayer%20Vehicle%20Reference) (+ (Variables|/Game/Callums_Stuff/OLDParent_BP.OLDParent_BP_C|GetRepair%20Kit%20Current (Variables|Default|GetPlayer%20Vehicle%20Reference)) (Variables|Default|GetVehicle%20Max%20-%20Current%20Difference)))
                  (Variables|Default|SetRepair%20Kit%20Station%20Stock%20Current (- (Variables|Default|GetRepair%20Kit%20Station%20Stock%20Current) (Variables|Default|GetVehicle%20Max%20-%20Current%20Difference))))))))
        (:then_1
          ;[1 1 1] New Vehicle
          (bind _asparent_vehicle_bp (Utilities|Casting|CastToParentVehicle_BP OtherActor))
          (Variables|Default|SetNew%20Player%20Vehicle%20Reference _asparent_vehicle_bp)
          (if (< (Variables|/Game/Army_Vehicles/ParentVehicle_BP.ParentVehicle_BP_C|GetRepair%20Kit%20Current (Variables|Default|GetNew%20Player%20Vehicle%20Reference)) (Variables|/Game/Army_Vehicles/ParentVehicle_BP.ParentVehicle_BP_C|GetRepair%20Kit%20Max (Variables|Default|GetNew%20Player%20Vehicle%20Reference)))
            (if (not (<= (Variables|Default|GetRepair%20Kit%20Station%20Stock%20Current) 0.0))
              (Variables|Default|SetVehicle%20Max%20-%20Current%20Difference (- (Variables|/Game/Army_Vehicles/ParentVehicle_BP.ParentVehicle_BP_C|GetRepair%20Kit%20Max (Variables|Default|GetNew%20Player%20Vehicle%20Reference)) (Variables|/Game/Army_Vehicles/ParentVehicle_BP.ParentVehicle_BP_C|GetRepair%20Kit%20Current (Variables|Default|GetNew%20Player%20Vehicle%20Reference))))
              (if (< (- (Variables|Default|GetRepair%20Kit%20Station%20Stock%20Current) (Variables|Default|GetVehicle%20Max%20-%20Current%20Difference)) 0.0)
                (Variables|/Game/Army_Vehicles/ParentVehicle_BP.ParentVehicle_BP_C|SetRepair%20Kit%20Current (Variables|Default|GetNew%20Player%20Vehicle%20Reference) (+ (Variables|Default|GetRepair%20Kit%20Station%20Stock%20Current) (Variables|/Game/Army_Vehicles/ParentVehicle_BP.ParentVehicle_BP_C|GetRepair%20Kit%20Current (Variables|Default|GetNew%20Player%20Vehicle%20Reference))))
                (Variables|Default|SetRepair%20Kit%20Station%20Stock%20Current (- (Variables|Default|GetRepair%20Kit%20Station%20Stock%20Current) (Variables|Default|GetRepair%20Kit%20Station%20Stock%20Current)))
                (else
                  (Variables|/Game/Army_Vehicles/ParentVehicle_BP.ParentVehicle_BP_C|SetRepair%20Kit%20Current (Variables|Default|GetNew%20Player%20Vehicle%20Reference) (+ (Variables|/Game/Army_Vehicles/ParentVehicle_BP.ParentVehicle_BP_C|GetRepair%20Kit%20Current (Variables|Default|GetNew%20Player%20Vehicle%20Reference)) (Variables|Default|GetVehicle%20Max%20-%20Current%20Difference)))
                  (Variables|Default|SetRepair%20Kit%20Station%20Stock%20Current (- (Variables|Default|GetRepair%20Kit%20Station%20Stock%20Current) (Variables|Default|GetVehicle%20Max%20-%20Current%20Difference))))))))))))

(event OnComponentEndOverlap(Box)
  (params (OverlappedComponent :type Primitive%20Component%20Object%20Reference) (OtherActor :type Actor%20Object%20Reference) (OtherComp :type Primitive%20Component%20Object%20Reference) (OtherBodyIndex :type Integer))
  (Utilities|FlowControl|Sequence
    (:then_0
      (Utilities|Casting|CastToOLDParent_BP OtherActor))
    (:then_1
      (Utilities|Casting|CastToParentVehicle_BP OtherActor)))
  (Utilities|FlowControl|Sequence
    (:then_0
      (Utilities|FlowControl|DoOnce false) ; enters at Reset
    )))

(event EventBeginPlay)

(event Collision|EventActorBeginOverlap
  (params (OtherActor :type Actor%20Object%20Reference)))

(event EventTick
  (params (DeltaSeconds :type Float%20%28single-precision%29)))

(fn ConstructionScript)