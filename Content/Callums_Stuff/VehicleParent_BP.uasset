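; Base drivable vehicle, judging by its name, with four switchable cameras, horn, headlights, playlist music and speed-driven engine audio.
; Armour-scaled damage crosses thresholds to add smoke, disable, then explode the vehicle.
; Tick drains fuel while moving and cuts throttle when empty; incoming fuel fills the tank, then spare canisters, which refuel it on a looping timer.
; Repair kits restore health instantly; their repair timer changes nothing and the handbrake stays set.
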(event Custom|Disable%20Vehicle
  ;[1 1 1] Disable Vehicle
  (Variables|CarStates|SetIs%20Disabled true)
  (Class|WheeledVehicleMovementComponent|SetHandbrakeInput (Variables|Default|GetVehicleMovement) true))

(event Custom|Destroy%20Vehicle
  (bind _mesh (Variables|Character|GetMesh))
  (bind _returnvalue (Transformation|GetWorldLocation _mesh))
  ;[1 1 1] Destroy Vehicle
  (Variables|CarStates|SetIs%20Disabled true)
  (Variables|CarStates|SetIs%20Destroyed true)
  (Effects|SpawnEmitterAttached "/Game/StarterContent/Particles/P_Fire.P_Fire" (Variables|Default|GetFire%20Transform%20Point) "None" "0, 0, 0" "0, 0, 0" "5.000000,5.000000,5.000000")
  (Class|WheeledVehicleMovementComponent|SetHandbrakeInput (Variables|Default|GetVehicleMovement) true)
  (Utilities|FlowControl|Delay 5.0)
  (Effects|SpawnEmitteratLocation "/Game/StarterContent/Particles/P_Explosion.P_Explosion" _returnvalue "0, 0, 0" "10.000000,10.000000,10.000000")
  (Audio|PlaySoundatLocation "/Game/StarterContent/Audio/Explosion02.Explosion02" _returnvalue "0, 0, 0" 1.0 1.0 0.0 0 0 0)
  (Rendering|SetVisibility (Variables|Character|GetMesh) false false)
  (Utilities|FlowControl|Delay 5.0)
  (Actor|DestroyActor))

(event Custom|Start%20Fuel%20Timer
  ;[1 1 1] Refuel from Can Timer Events
  (Utilities|Time|SetTimerbyEvent (delegate Custom|Add%20Fuel) 0.01 true))

(event Custom|Add%20Fuel
  ;[1 1 1] Refuel from Can Timer Events
  (if (Variables|Refuelling|GetRefuelling%20From%20Can)
    (if (>= (Variables|FuelTank|GetCurrent%20Fuel%20Amount) (Variables|FuelTank|GetMaximum%20Fuel%20Capacity))
      (Class|WheeledVehicleMovementComponent|SetHandbrakeInput (Variables|Default|GetVehicleMovement) false :!label _label)
      (Variables|Refuelling|SetRefuelling%20From%20Can false)
      (elif (<= (Variables|FuelCanister|GetFuel%20Canister%20Current%20Fuel%20Amount) 0.0)
        (goto _label)
        (else
          (CallFunction|FuelEvent 1.0))))))

(event Custom|Damaged
  ;[1 1 1] Damage Vehicle
  (Variables|CarStates|SetIs%20Damaged true)
  (Effects|SpawnEmitterAttached "/Game/StarterContent/Particles/P_Smoke.P_Smoke" (Variables|Default|GetSmoke%20Transform%20Point) "None"))

(event Custom|Start%20Repair%20Timer
  (Utilities|Time|SetTimerbyEvent (delegate Custom|Add%20Health) 1.0 true))

(event Custom|Add%20Health
  (if (Variables|Default|GetIs%20Repairing)
    (if (>= (Variables|CarStats|GetCurrent%20Health) (Variables|CarStats|GetMaximum%20health))
      (if (<= (Variables|Default|GetRepair%20Kit%20Current) 0.0)
        _))))

(event EventBeginPlay)

(event EventHealth/DamageEvent
  (params (Damage%20Amount :type Float%20%28single-precision%29) (Bone%20Name :type Float%20%28single-precision%29))
  ;[1 1 1] Calculate Health on Health/Damage Event
  (CallFunction|CalculateHealth Damage%20Amount))

(event EventTick
  (params (DeltaSeconds :type Float%20%28single-precision%29))
  (bind _vehiclemovement (Variables|Default|GetVehicleMovement))
  (bind _returnvalue (Class|WheeledVehicleMovementComponent|GetForwardSpeed _vehiclemovement))
  (Utilities|FlowControl|Sequence
    (:then_0
      ;[1 1 1] Play Engine Sound
      (Audio|Parameter|SetFloatParameter (Variables|Default|GetEngine%20Sound) "RPM" (Math|Float|Absolute(Float) (Class|WheeledVehicleMovementComponent|GetForwardSpeed (Variables|Default|GetVehicleMovement))) :!class /Script/Engine.AudioComponent))
    (:then_1
      ;[1 1 1] Fuel Consumption
      (if (or (>= _returnvalue 5.0) (<= _returnvalue -5.0))
        (Variables|FuelTank|SetCurrent%20Fuel%20Amount (- (Variables|FuelTank|GetCurrent%20Fuel%20Amount) 1.0))
        (if (<= (Variables|FuelTank|GetCurrent%20Fuel%20Amount) 0.0)
          (Variables|FuelTank|SetCurrent%20Fuel%20Amount 0.0)
          (Class|WheeledVehicleMovementComponent|SetThrottleInput (Variables|Default|GetVehicleMovement) 0.0))))))

(event EventFuelEvent
  (params (Fuel%20Amount :type Float%20%28single-precision%29))
  ;[1 1 1] Calculate Fuel on Fuel Event
  (CallFunction|CalculateFuel Fuel%20Amount)
  (Development|PrintString (Utilities|String|ToString(Float) (Variables|FuelCanister|GetCurrent%20Fuel%20Canisters%20Held%20)))
  (Development|PrintString (Utilities|String|ToString(Float) (Variables|FuelCanister|GetFuel%20Canister%20Current%20Fuel%20Amount)) true true "(R=1.000000,G=0.193417,B=0.013272,A=1.000000)"))

(event Input|ActionEvents|InputActionActivateCamera2
  (params (Key :type Key%20Structure :default "None"))
  ;[1 1 1] Camera Switching
  ;;[1 1 1] Specific Camera Switching
  (:Pressed
    (Components|Activation|SetActive (Variables|Default|GetThird%20Person%20Camera) true false)
    (Components|Activation|SetActive (Variables|Components|GetFirst%20Person%20Camera) false false)
    (Components|Activation|SetActive (Variables|Default|GetBumper%20Camera) false false)
    (Components|Activation|SetActive (Variables|Default|GetSide%20Camera) false false)
    (Variables|Default|SetCamera%20Integer 2)))

(event Input|ActionEvents|InputActionManualRefuel
  (params (Key :type Key%20Structure :default "None"))
  (bind _vehiclemovement (Variables|Default|GetVehicleMovement))
  ;[1 1 1] manual refuel
  (:Pressed
    (Utilities|FlowControl|FlipFlop
      (:A
        (if (== (Class|WheeledVehicleMovementComponent|GetForwardSpeed _vehiclemovement) 0.0)
          (if (>= (Variables|FuelCanister|GetFuel%20Canister%20Current%20Fuel%20Amount) 1.0)
            (if (< (Variables|FuelTank|GetCurrent%20Fuel%20Amount) (Variables|FuelTank|GetMaximum%20Fuel%20Capacity))
              (Class|WheeledVehicleMovementComponent|SetHandbrakeInput (Variables|Default|GetVehicleMovement) true)
              (CallFunction|StartFuelTimer)
              (Variables|Refuelling|SetRefuelling%20From%20Can true)
              (Development|PrintString "refuelling")))))
      (:B
        (Class|WheeledVehicleMovementComponent|SetHandbrakeInput _vehiclemovement false)
        (Variables|Refuelling|SetRefuelling%20From%20Can false)))))

(event Input|ActionEvents|InputActionNextSong
  (params (Key :type Key%20Structure :default "None"))
  (:Pressed
    (Class|MediaPlayer|Next (Variables|Default|GetMedia%20Player))
    (Variables|Default|SetSong%20Number (+ (Variables|Default|GetSong%20Number) 1))))

(event Input|ActionEvents|InputActionPreviousSong
  (params (Key :type Key%20Structure :default "None"))
  (:Pressed
    (Class|MediaPlayer|Previous (Variables|Default|GetMedia%20Player))
    (Variables|Default|SetSong%20Number (- (Variables|Default|GetSong%20Number) 1))
    (if (<= (Variables|Default|GetSong%20Number) 0)
      (Variables|Default|SetSong%20Number 0))))

(event Input|ActionEvents|InputActionActivateCamera3
  (params (Key :type Key%20Structure :default "None"))
  ;[1 1 1] Camera Switching
  ;;[1 1 1] Specific Camera Switching
  (:Pressed
    (Components|Activation|SetActive (Variables|Default|GetBumper%20Camera) true false)
    (Components|Activation|SetActive (Variables|Components|GetFirst%20Person%20Camera) false false)
    (Components|Activation|SetActive (Variables|Default|GetThird%20Person%20Camera) false false)
    (Components|Activation|SetActive (Variables|Default|GetSide%20Camera) false false)
    (Variables|Default|SetCamera%20Integer 3)))

(event Input|ActionEvents|InputActionActivateCamera4
  (params (Key :type Key%20Structure :default "None"))
  ;[1 1 1] Camera Switching
  ;;[1 1 1] Specific Camera Switching
  (:Pressed
    (Components|Activation|SetActive (Variables|Default|GetSide%20Camera) true false)
    (Components|Activation|SetActive (Variables|Components|GetFirst%20Person%20Camera) false false)
    (Components|Activation|SetActive (Variables|Default|GetThird%20Person%20Camera) false false)
    (Components|Activation|SetActive (Variables|Default|GetBumper%20Camera) false false)
    (Variables|Default|SetCamera%20Integer 0)))

(event Input|ActionEvents|InputActionSwitchCamera
  (params (Key :type Key%20Structure :default "None"))
  ;[1 1 1] Camera Switching
  ;;[1 1 1] Toggle Camera Switching
  (:Pressed
    (switch int (Variables|Default|GetCamera%20Integer)
      (:0
        (Components|Activation|SetActive (Variables|Components|GetFirst%20Person%20Camera) true false)
        (Components|Activation|SetActive (Variables|Default|GetThird%20Person%20Camera) false false)
        (Components|Activation|SetActive (Variables|Default|GetBumper%20Camera) false false)
        (Components|Activation|SetActive (Variables|Default|GetSide%20Camera) false false)
        (Variables|Default|SetCamera%20Integer 1))
      (:1
        (Components|Activation|SetActive (Variables|Default|GetThird%20Person%20Camera) true false)
        (Components|Activation|SetActive (Variables|Components|GetFirst%20Person%20Camera) false false)
        (Components|Activation|SetActive (Variables|Default|GetBumper%20Camera) false false)
        (Components|Activation|SetActive (Variables|Default|GetSide%20Camera) false false)
        (Variables|Default|SetCamera%20Integer 2))
      (:2
        (Components|Activation|SetActive (Variables|Default|GetBumper%20Camera) true false)
        (Components|Activation|SetActive (Variables|Components|GetFirst%20Person%20Camera) false false)
        (Components|Activation|SetActive (Variables|Default|GetThird%20Person%20Camera) false false)
        (Components|Activation|SetActive (Variables|Default|GetSide%20Camera) false false)
        (Variables|Default|SetCamera%20Integer 3))
      (:3
        (Components|Activation|SetActive (Variables|Default|GetSide%20Camera) true false)
        (Components|Activation|SetActive (Variables|Components|GetFirst%20Person%20Camera) false false)
        (Components|Activation|SetActive (Variables|Default|GetThird%20Person%20Camera) false false)
        (Components|Activation|SetActive (Variables|Default|GetBumper%20Camera) false false)
        (Variables|Default|SetCamera%20Integer 0)))))

(event Input|ActionEvents|InputActionActivateCamera1
  (params (Key :type Key%20Structure :default "None"))
  ;[1 1 1] Camera Switching
  ;;[1 1 1] Specific Camera Switching
  (:Pressed
    (Components|Activation|SetActive (Variables|Components|GetFirst%20Person%20Camera) true false)
    (Components|Activation|SetActive (Variables|Default|GetThird%20Person%20Camera) false false)
    (Components|Activation|SetActive (Variables|Default|GetBumper%20Camera) false false)
    (Components|Activation|SetActive (Variables|Default|GetSide%20Camera) false false)
    (Variables|Default|SetCamera%20Integer 1)))

(event Input|ActionEvents|InputActionHorn
  (params (Key :type Key%20Structure :default "None"))
  ;[1 1 1] Horn
  (:Pressed
    (Audio|PlaySoundatLocation (Variables|Default|GetHorn%20Sound) (Transformation|GetWorldLocation (Variables|Character|GetMesh)) "0, 0, 0" 1.0 1.0 0.0 0 0 0)))

(event Input|ActionEvents|InputActionManualRepair
  (params (Key :type Key%20Structure :default "None"))
  (:Pressed
    (if (== (Class|WheeledVehicleMovementComponent|GetForwardSpeed (Variables|Default|GetVehicleMovement)) 0.0)
      (if (< (Variables|CarStats|GetCurrent%20Health) (Variables|CarStats|GetMaximum%20health))
        (if (>= (Variables|Default|GetRepair%20Kit%20Current) 1.0)
          (Class|WheeledVehicleMovementComponent|SetHandbrakeInput (Variables|Default|GetVehicleMovement) true)
          (CallFunction|StartRepairTimer)
          (Variables|Default|SetIs%20Repairing true)
          (Variables|CarStats|SetCurrent%20Health (+ (Variables|CarStats|GetCurrent%20Health) (Variables|Default|GetRepair%20Kit%20Max%20Health%20Restored)))
          (Variables|Default|SetRepair%20Kit%20Current (- (Variables|Default|GetRepair%20Kit%20Current) 1.0)))))))

(event Input|ActionEvents|InputActionActivateLights
  (params (Key :type Key%20Structure :default "None"))
  ;[1 1 1] Turn Headlights On/Off
  (:Pressed
    (Utilities|FlowControl|FlipFlop
      (:A
        (Rendering|SetVisibility (Variables|Default|GetLeft%20Headlight) true false)
        (Rendering|SetVisibility (Variables|Default|GetRight%20Headlight) true false))
      (:B
        (Rendering|SetVisibility (Variables|Default|GetLeft%20Headlight) false false)
        (Rendering|SetVisibility (Variables|Default|GetRight%20Headlight) false false)))))

(event Input|ActionEvents|InputActionPlayMusic
  (params (Key :type Key%20Structure :default "None"))
  (bind _media_player (Variables|Default|GetMedia%20Player))
  (:Pressed
    (if (Variables|Default|GetMusic%20Is%20Playing)
      (Sequencer|Player|Pause _media_player)
      (Variables|Default|SetMusic%20Is%20Playing false)
      (else
        (Class|MediaPlayer|OpenPlaylistIndex _media_player "/Game/Callums_Stuff/MusicNonsense/SongPlaylist.SongPlaylist" (Variables|Default|GetSong%20Number))
        (Variables|Default|SetMusic%20Is%20Playing true)))))

(event Input|AxisEvents|InputAxisMoveForward
  (params (AxisValue :type Float%20%28single-precision%29))
  (if (not (<= (Variables|FuelTank|GetCurrent%20Fuel%20Amount) 0.0))
    (Class|WheeledVehicleMovementComponent|SetThrottleInput (Variables|Default|GetVehicleMovement) AxisValue)))

(event Input|AxisEvents|InputAxisMoveRight
  (params (AxisValue :type Float%20%28single-precision%29))
  (Class|WheeledVehicleMovementComponent|SetSteeringInput (Variables|Default|GetVehicleMovement) AxisValue))

(event Input|AxisEvents|InputAxisLookUp
  (params (AxisValue :type Float%20%28single-precision%29))
  (bind _returnvalue (Input|AxisValues|GetLookRight))
  (bind _returnvalue_2 (Input|AxisValues|GetLookUp))
  (bind _first_person_spring_arm (Variables|Components|GetFirst%20Person%20Spring%20Arm))
  (bind _relativerotation (Variables|/Script/Engine.SceneComponent|GetRelativeRotation _first_person_spring_arm))
  (bind (_roll _pitch _yaw) (Math|Rotator|BreakRotator _relativerotation))
  (bind _returnvalue_3 (+ _returnvalue_2 _pitch))
  (bind _returnvalue_4 (+ _yaw _returnvalue))
  (bind _returnvalue_5 (Math|Float|ClampAngle _returnvalue_3 -89.0 89.0))
  (bind _returnvalue_6 (Math|Rotator|MakeRotator 0.0 _returnvalue_5 _returnvalue_4))
  ;[1 1 1] Rotate First Person Camera
  (Pawn|Input|AddControllerPitchInput (* AxisValue -1.0))
  (Transformation|SetRelativeRotation (Variables|Components|GetFirst%20Person%20Spring%20Arm) _returnvalue_6 false false)
  (Transformation|SetRelativeRotation (Variables|Default|GetThird%20Person%20Spring%20Arm) _returnvalue_6 false false)
  (Transformation|SetRelativeRotation (Variables|Default|GetSide%20Camera%20Spring%20Arm) _returnvalue_6 false false))

(event Input|AxisEvents|InputAxisMoveRight
  (params (AxisValue :type Float%20%28single-precision%29))
  (bind _returnvalue (Input|AxisValues|GetLookRight))
  (bind _returnvalue_2 (Input|AxisValues|GetLookUp))
  (bind _first_person_spring_arm (Variables|Components|GetFirst%20Person%20Spring%20Arm))
  (bind _relativerotation (Variables|/Script/Engine.SceneComponent|GetRelativeRotation _first_person_spring_arm))
  (bind (_roll _pitch _yaw) (Math|Rotator|BreakRotator _relativerotation))
  (bind _returnvalue_3 (+ _returnvalue_2 _pitch))
  (bind _returnvalue_4 (+ _yaw _returnvalue))
  (bind _returnvalue_5 (Math|Float|ClampAngle _returnvalue_3 -89.0 89.0))
  (bind _returnvalue_6 (Math|Rotator|MakeRotator 0.0 _returnvalue_5 _returnvalue_4))
  ;[1 1 1] Rotate First Person Camera
  (Pawn|Input|AddControllerYawInput AxisValue)
  (Transformation|SetRelativeRotation (Variables|Components|GetFirst%20Person%20Spring%20Arm) _returnvalue_6 false false)
  (Transformation|SetRelativeRotation (Variables|Default|GetThird%20Person%20Spring%20Arm) _returnvalue_6 false false)
  (Transformation|SetRelativeRotation (Variables|Default|GetSide%20Camera%20Spring%20Arm) _returnvalue_6 false false))

(event Input|KeyboardEvents|SpaceBar
  (params (Key :type Key%20Structure :default "None"))
  (bind _vehiclemovement (Variables|Default|GetVehicleMovement))
  (:Pressed
    (Class|WheeledVehicleMovementComponent|SetHandbrakeInput _vehiclemovement true))
  (:Released
    (if (not (Variables|CarStates|GetIs%20Disabled))
      (Class|WheeledVehicleMovementComponent|SetHandbrakeInput _vehiclemovement false))))

(event Input|MouseEvents|LeftMouseButton
  (params (Key :type Key%20Structure :default "None")))

(fn ConstructionScript)

(fn CalculateHealth
  (params (Damage%20Amount :type Float%20%28single-precision%29))
  (Variables|CarStats|SetCurrent%20Health (- (Variables|CarStats|GetCurrent%20Health) (* Damage%20Amount (Variables|CarStats|GetArmour))))
  (if (<= (Variables|CarStats|GetCurrent%20Health) (Variables|CarStats|GetDamage%20Warning%20Threshold))
    (CallFunction|Damaged)
    (if (<= (Variables|CarStats|GetCurrent%20Health) (Variables|CarStats|GetDisabled%20Threshold))
      (CallFunction|DisableVehicle)
      (if (<= (Variables|CarStats|GetCurrent%20Health) (Variables|CarStats|GetDestroyed%20Threshold))
        (CallFunction|DestroyVehicle)))))

(fn CalculateFuel
  (params (Incoming%20Fuel%20Amount :type Float%20%28single-precision%29))
  (Variables|Refuelling|SetIncoming%20Fuel%20Amount Incoming%20Fuel%20Amount)
  (if (Variables|Refuelling|GetRefuelling%20From%20Can)
    ;[1 1 1] Add Fuel to Tank from fuel cans
    ;;[1 1 1] Subtract Fuel From Fuel Canisters
    (Variables|FuelCanister|SetFuel%20Canister%20Current%20Fuel%20Amount (- (Variables|FuelCanister|GetFuel%20Canister%20Current%20Fuel%20Amount) (Variables|Refuelling|GetIncoming%20Fuel%20Amount)))
    (Utilities|FlowControl|Sequence
      (:then_0
        ;;[1 1 1] Add Fuel
        (Variables|FuelTank|SetCurrent%20Fuel%20Amount (+ (Variables|Refuelling|GetIncoming%20Fuel%20Amount) (Variables|FuelTank|GetCurrent%20Fuel%20Amount)))
        (if (>= (Variables|FuelTank|GetCurrent%20Fuel%20Amount) (Variables|FuelTank|GetMaximum%20Fuel%20Capacity))
          (Variables|FuelTank|SetCurrent%20Fuel%20Amount (Variables|FuelTank|GetMaximum%20Fuel%20Capacity))))
      (:then_1
        ;;[1 1 1] Fuel Canister Total Subtraction and other calculations
        (if (<= (Variables|FuelCanister|GetFuel%20Canister%20Current%20Fuel%20Amount) 0.0)
          (if (not (== (Variables|FuelCanister|GetCurrent%20Fuel%20Canisters%20Held%20) 0.0))
            (Variables|FuelCanister|SetCurrent%20Fuel%20Canisters%20Held%20 (- (Variables|FuelCanister|GetCurrent%20Fuel%20Canisters%20Held%20) 1.0))
            (if (and (<= (Variables|FuelCanister|GetFuel%20Canister%20Current%20Fuel%20Amount) 0.0) (>= (Variables|FuelCanister|GetCurrent%20Fuel%20Canisters%20Held%20) 1.0))
              (Variables|FuelCanister|SetFuel%20Canister%20Current%20Fuel%20Amount (Variables|FuelCanister|GetFuel%20Canister%20Maximum%20Capacity)))))))
    (elif (< (Variables|FuelTank|GetCurrent%20Fuel%20Amount) (Variables|FuelTank|GetMaximum%20Fuel%20Capacity))
      ;[1 1 1] Add Fuel To Tank
      (Variables|FuelTank|SetCurrent%20Fuel%20Amount (+ (Variables|Refuelling|GetIncoming%20Fuel%20Amount) (Variables|FuelTank|GetCurrent%20Fuel%20Amount)))
      (if (>= (Variables|FuelTank|GetCurrent%20Fuel%20Amount) (Variables|FuelTank|GetMaximum%20Fuel%20Capacity))
        (Variables|FuelTank|SetCurrent%20Fuel%20Amount (Variables|FuelTank|GetMaximum%20Fuel%20Capacity)))
      (else
        ;[1 1 1] Add Fuel to Fuel Cans
        (if (< (Variables|FuelCanister|GetCurrent%20Fuel%20Canisters%20Held%20) (Variables|FuelCanister|GetFuel%20Canisters%20Held%20Maximum))
          (Variables|FuelCanister|SetFuel%20Canister%20Current%20Fuel%20Amount (+ (Variables|FuelCanister|GetFuel%20Canister%20Current%20Fuel%20Amount) (Variables|Refuelling|GetIncoming%20Fuel%20Amount)))
          (if (>= (Variables|FuelCanister|GetFuel%20Canister%20Current%20Fuel%20Amount) (Variables|FuelCanister|GetFuel%20Canister%20Maximum%20Capacity))
            (Variables|FuelCanister|SetCurrent%20Fuel%20Canisters%20Held%20 (+ (Variables|FuelCanister|GetCurrent%20Fuel%20Canisters%20Held%20) 1.0))
            (if (>= (Variables|FuelCanister|GetCurrent%20Fuel%20Canisters%20Held%20) (Variables|FuelCanister|GetFuel%20Canisters%20Held%20Maximum))
              (Variables|FuelCanister|SetFuel%20Canister%20Current%20Fuel%20Amount (Variables|FuelCanister|GetFuel%20Canister%20Maximum%20Capacity))
              (else
                (Variables|FuelCanister|SetFuel%20Canister%20Current%20Fuel%20Amount 0.0)))))))))